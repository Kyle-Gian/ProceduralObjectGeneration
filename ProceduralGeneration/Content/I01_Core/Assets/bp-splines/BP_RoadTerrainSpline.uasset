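; Spline-based road actor that builds a mesh road and can snap its spline to the surface beneath it.
; CreateRoad adds one scaled spline mesh per segment, using world-space point positions and tangents.
; EditorRalignSpline line-traces vertically through each point and sets it slightly above the hit.
; DeformLandscape and RealignSplineOverDistance are empty stubs, and the landscape EditorApplySpline call is unconnected.
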(event Custom|DeformLandscape)

(event Custom|CreateRoad
  (bind _mesh_scale (Variables|Default|GetMesh%20Scale))
  (bind _spline (Variables|Default|GetSpline))
  (Utilities|Array|Clear (Variables|Default|GetSplineMeshList))
  (for _index (range 0 (- (Spline|GetNumberOfSplinePoints (Variables|Default|GetSpline)) 2))
    (bind _returnvalue (AddComponent|AddSplineMeshComponent false))
    (Utilities|Array|Add (Variables|Default|GetSplineMeshList) _returnvalue)
    (SplineMesh|SetStartScale _returnvalue _mesh_scale true :!class /Script/Engine.SplineMeshComponent)
    (SplineMesh|SetEndScale _returnvalue _mesh_scale true :!class /Script/Engine.SplineMeshComponent)
    (SplineMesh|SetStartandEnd _returnvalue (Spline|GetLocationatSplinePoint _spline _index "World") (Spline|GetTangentatSplinePoint _spline _index "World") (Spline|GetLocationatSplinePoint _spline (+ _index 1) "World") (Spline|GetTangentatSplinePoint _spline (+ _index 1) "World") true :!class /Script/Engine.SplineMeshComponent)))

(event Custom|EditorRalignSpline
  (CallFunction|RealignSplinewithPoints))

(event EventBeginPlay)

(event Collision|EventActorBeginOverlap
  (params (OtherActor :type Actor%20Object%20Reference)))

(event EventTick
  (params (DeltaSeconds :type Float%20%28single-precision%29)))

(fn ConstructionScript)

(fn RealignSplinewithPoints
  (bind _spline (Variables|Default|GetSpline))
  (for _index (range 0 (- (Spline|GetNumberOfSplinePoints _spline) 1))
    (bind (_outhit _returnvalue) (Collision|LineTraceByChannel (+ (Spline|GetLocationatSplinePoint _spline _index "World") "0,0,500.000000") (- (Spline|GetLocationatSplinePoint _spline _index "World") "0,0,500.000000") "TraceTypeQuery1" true 0 "ForDuration"))
    (if _returnvalue
      (Development|PrintString (Utilities|GetDisplayName (.HitActor (Collision|BreakHitResult _outhit))))
      (Spline|SetLocationatSplinePoint (Variables|Default|GetSpline) _index (Math|Vector|MakeVector (.x (Spline|GetLocationatSplinePoint (Variables|Default|GetSpline) _index "World")) (.y (Spline|GetLocationatSplinePoint (Variables|Default|GetSpline) _index "World")) (+ (.Z (Math|Vector|BreakVector (.ImpactPoint (Collision|BreakHitResult _outhit)))) 1e+01)) "World" true))))

(fn RealignSplineOverDistance)