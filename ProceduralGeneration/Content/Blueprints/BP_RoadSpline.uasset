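; BP_RoadSpline is a spline-based road actor that builds road geometry and can deform the landscape to match it.
; The construction script runs CreateRoad, which clears old segments and adds a collision-enabled spline mesh, a scaled cube, between each pair of neighboring points.
; A separate DeformLandscape event applies the same spline to the landscape through EditorApplySpline, using configurable width, falloff and subdivisions.
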(event Custom|DeformLandscape
  (bind _side_falloff (Variables|Default|GetSide%20Falloff))
  (bind _roadwidth (Variables|Default|GetRoadWidth))
  (Landscape|Editor|EditorApplySpline (Variables|Default|GetLandScape) (Variables|Default|GetSpline) _roadwidth _roadwidth _side_falloff _side_falloff 0.0 0.0 (Variables|Default|GetNum%20Subdivisions) true true 0 "None"))

(event Custom|CreateRoad
  (bind _spline (Variables|Default|GetSpline))
  (bind _spline_2 (Variables|Default|GetSpline))
  (bind _meshscale (Variables|Default|GetMeshScale))
  (for _array_element (Variables|Default|GetSplineMeshList)
    (Components|DestroyComponent _array_element))
  (Utilities|Array|Clear (Variables|Default|GetSplineMeshList))
  (for _index (range 0 (- (Spline|GetNumberOfSplinePoints (Variables|Default|GetSpline)) 2))
    (bind _returnvalue (AddComponent|AddSplineMeshComponent false))
    (Utilities|Array|Add (Variables|Default|GetSplineMeshList) _returnvalue)
    (Components|StaticMesh|SetStaticMesh _returnvalue "/Game/Geometry/Meshes/1M_Cube.1M_Cube")
    (SplineMesh|SetStartScale _returnvalue _meshscale true :!class /Script/Engine.SplineMeshComponent)
    (SplineMesh|SetEndScale _returnvalue _meshscale true :!class /Script/Engine.SplineMeshComponent)
    (SplineMesh|SetStartandEnd _returnvalue (Spline|GetLocationatSplinePoint _spline _index "Local") (Spline|GetTangentatSplinePoint _spline _index "Local") (Spline|GetLocationatSplinePoint _spline_2 (+ _index 1) "Local") (Spline|GetTangentatSplinePoint _spline_2 (+ _index 1) "Local") true :!class /Script/Engine.SplineMeshComponent)
    (Collision|SetCollisionEnabled _returnvalue "QueryAndPhysics")))

(event EventBeginPlay)

(fn ConstructionScript
  (CallFunction|CreateRoad))